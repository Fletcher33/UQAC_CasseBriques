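; BP_Wall is a wall actor meant to bounce BP_Ball according to its Type.
; On overlap it only casts the other actor to BP_Ball, as the bounce logic is disconnected and never runs.
; That unused logic negates the ball sphere's Y velocity for Gauche and Droite walls or X for Haut, then prints velocity and Type.
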(event `self.ReceiveActorBeginOverlap`
  (params (OtherActor :type "Actor Object Reference"))
  (bind _asbp_ball (cast `/Game/Actors/BP_Ball` OtherActor)))

(fn `UserConstructionScript`)