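; BP_Paddle is a player-controlled paddle that moves along world Y from the Horizontal input axis and deflects BP_Ball.
; When a ball stops overlapping the paddle, it sets the ball sphere's physics velocity with a fixed positive X speed and a computed Y.
; GenerateYVelocity keeps whichever Y velocity has the larger magnitude, paddle or ball, with its sign intact.
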(event `InputAxis|Horizontal`
  (params (AxisValue :type "Float (single-precision)"))
  (`self.AddMovementInput` (0.0 1.0 0.0) AxisValue))

(event `self.ReceiveActorEndOverlap`
  (params (OtherActor :type "Actor Object Reference"))
  (bind (_returnvalue_x _returnvalue_y) (`KismetMathLibrary.BreakVector` (`SceneComponent.GetComponentVelocity` (`self.Cube`))))
  (bind _asbp_ball (cast `/Game/Actors/BP_Ball` OtherActor))
  (bind _new_y (`self.Generate Y velocity` _returnvalue_y _asbp_ball))
  (`PrimitiveComponent.SetPhysicsLinearVelocity` (`/Game/Actors/BP_Ball.Sphere` _asbp_ball) (`KismetMathLibrary.MakeVector` 1000.0 _new_y) false "None"))

(fn `Generate Y velocity`
  (params (`Paddle Y velocity` :type "Float (double-precision)") (Ball :type "/Game/Actors/BP_Ball Object Reference"))
  (returns (`New Y` :type "Float (double-precision)"))
  (bind (_returnvalue_x _returnvalue_y) (`KismetMathLibrary.BreakVector` (`self.GetVelocity` Ball)))
  (bind _paddle_y_velocity (`local.Paddle Y velocity`))
  (if (> `Paddle Y velocity` 0.0)
    (set `self.PaddleSign` 1.0)
    (else
      (set `self.PaddleSign` -1.0)))
  (if (> _returnvalue_y 0.0)
    (set `self.BallSign` 1.0)
    (else
      (set `self.BallSign` -1.0)))
  (if (> (* _paddle_y_velocity (`self.PaddleSign`)) (* _returnvalue_y (`self.BallSign`)))
    (return _paddle_y_velocity)
    (else
      (return _returnvalue_y))))

(fn `UserConstructionScript`)