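; BP_Ball is a physics-driven ball actor that launches along negative X at BeginPlay and resets its score to zero.
; Tick prints the sphere's velocity and the score, which nothing here increments.
; Bounce logic for BP_Wall and BP_Paddle, scaling velocity by the paddle's VelocityModifier even for walls, is disconnected and never runs, leaving the overlap event empty.
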(event `self.ReceiveBeginPlay`
  (set `self.Score` 0)
  (`PrimitiveComponent.SetPhysicsLinearVelocity` (`self.Sphere`) (-1000.0 0.0 0.0) false "None"))

(event `self.ReceiveActorBeginOverlap`
  (params (OtherActor :type "Actor Object Reference")))

(event `self.ReceiveTick`
  (params (DeltaSeconds :type "Float (single-precision)"))
  (`KismetSystemLibrary.PrintString` (`KismetStringLibrary.Conv_VectorToString` (`SceneComponent.GetComponentVelocity` (`self.Sphere`))))
  (`KismetSystemLibrary.PrintString` (`KismetStringLibrary.Conv_IntToString` (`self.Score`))))

(fn `UserConstructionScript`)