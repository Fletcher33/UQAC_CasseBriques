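; Breakout-style brick actor that loses one HP each time a BP_Ball ends overlap with it.
; BeginPlay rolls a random HP from zero to three through nested chance checks, weighted toward higher values, so some bricks vanish immediately.
; UpdateColor maps remaining HP to the cube's material and destroys the brick at zero, adding a point to the ball's Score only when a hit caused it.
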(event `self.ReceiveActorEndOverlap`
  (params (OtherActor :type "Actor Object Reference"))
  (bind _asbp_ball (cast `/Game/Actors/BP_Ball` OtherActor))
  (set `self.HP` (+ (`self.HP`) -1))
  (`self.Update_Color` true _asbp_ball))

(event `self.ReceiveBeginPlay`
  (`self.Setup_Random_HP`)
  (`self.Update_Color` false))

(fn `Setup_Random_HP`
  (bind _returnvalue (`KismetMathLibrary.RandomInteger` 100))
  (if (> _returnvalue 90)
    (set `self.HP` 0)
    (elif (> _returnvalue 80)
      (set `self.HP` 1)
      (elif (> _returnvalue 60)
        (set `self.HP` 2)
        (else
          (set `self.HP` 3))))))

(fn `Update_Color`
  (params (Points :type Boolean) (Balle :type "/Game/Actors/BP_Ball Object Reference"))
  (bind _cube (`self.Cube`))
  (switch `int` (`self.HP`)
    (:`0`
      (`self.K2_DestroyActor`)
      (if Points
        (set `/Game/Actors/BP_Ball.Score` (+ (`/Game/Actors/BP_Ball.Score` Balle) 1) Balle)))
    (:`1`
      (`PrimitiveComponent.SetMaterial` _cube 0 "/Game/Materials/Red.Red"))
    (:`2`
      (`PrimitiveComponent.SetMaterial` _cube 0 "/Game/Materials/Orange.Orange"))
    (:`3`
      (`PrimitiveComponent.SetMaterial` _cube 0 "/Game/Materials/Green.Green"))))

(fn `UserConstructionScript`)